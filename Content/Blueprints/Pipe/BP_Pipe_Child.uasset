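; Child pipe Blueprint for a throwable pipe that sticks into tagged surfaces.
; When projectile movement stops on an actor tagged "ForPipe", it snaps to the impact point along the surface normal, becomes WorldStatic and disables its grab box.
; On any other hit it prints a debug message and teleports to the Respawn1 position with a random Y offset.
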(event OnProjectileStop(ProjectileMovement)
  (params (ImpactResult :type Hit%20Result%20Structure%20%28by%20ref%29))
  (bind _respawn1 (Variables|Default|GetRespawn1))
  ;[0 0 0] OnProjectileStop
  (if (Actor|ActorHasTag (.hitactor ImpactResult) "ForPipe")
    (Transformation|SetActorLocationAndRotation (.impactpoint ImpactResult) (Math|Conversions|RotationFromXVector (.impactnormal ImpactResult)))
    (Variables|Default|SetstickedToWall? true)
    (Collision|SetCollisionObjectType (Variables|Default|GetPipe) "ECC_WorldStatic")
    (Collision|SetCollisionEnabled (Variables|Default|GetGrabBox) "NoCollision")
    (else
      (Development|PrintString "Non colpito")
      (Transformation|SetActorLocationAndRotation (Math|Vector|MakeVector (.x _respawn1) (Math|Random|RandomFloatinRange (- (.y _respawn1) 3e+02) (+ (.y _respawn1) 3e+02)) (.z _respawn1)) "0, 0, 0"))))

(event EventBeginPlay
  (|CallParentFunction))

(fn ConstructionScript
  (|CallParentFunction))