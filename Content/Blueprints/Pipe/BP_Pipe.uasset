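; BP_Pipe is a pipe actor that players can grab and that sticks into surfaces when its projectile movement stops.
; GrabBox overlaps notify the locally controlled BP_Player and toggle a tap-to-grab widget, shown only while the pipe is free and the player is empty-handed.
; On projectile stop, it aligns to the impact normal, becomes WorldStatic and disables GrabBox so it cannot be grabbed again.
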(event OnComponentBeginOverlap(GrabBox)
  (params (OverlappedComponent :type Primitive%20Component%20Object%20Reference) (OtherActor :type Actor%20Object%20Reference) (OtherComp :type Primitive%20Component%20Object%20Reference) (OtherBodyIndex :type Integer) (bFromSweep :type Boolean) (SweepResult :type Hit%20Result%20Structure%20%28by%20ref%29))
  ;[0 0 0] OnComponentBeginOverlap
  (if (not (Variables|Default|GetisGrabbed?))
    (if (not (Variables|Default|GetstickedToWall?))
      (bind _asbp_player (Utilities|Casting|CastToBP_Player OtherActor))
      (if (Pawn|IsLocallyControlled _asbp_player)
        (if (not (Variables|/Game/Characters/BP_Player.BP_Player_C|GetisHoldingPipe? _asbp_player))
          (Class|BPIPipe|SetPipeIntercation(Message) OtherActor self true)
          (Utilities|IsValid (Variables|Default|GetWB_TapToGrab)
            (:Is%20Valid
              _)
            (:Is%20Not%20Valid
              (bind _returnvalue (UserInterface|CreateWidget "/Game/Widget/WB_TapEToGrab.WB_TapEToGrab_C" (Pawn|GetLocalViewingPlayerController _asbp_player)))
              (Variables|Default|SetWB_TapToGrab _returnvalue)))
          (UserInterface|Viewport|AddtoViewport (Variables|Default|GetWB_TapToGrab) 0))))))

(event OnComponentEndOverlap(GrabBox)
  (params (OverlappedComponent :type Primitive%20Component%20Object%20Reference) (OtherActor :type Actor%20Object%20Reference) (OtherComp :type Primitive%20Component%20Object%20Reference) (OtherBodyIndex :type Integer))
  ;[0 0 0] OnComponentEndOverlap
  (bind _asbp_player (Utilities|Casting|CastToBP_Player OtherActor))
  (if (Pawn|IsLocallyControlled _asbp_player)
    (Class|BPIPipe|SetPipeIntercation(Message) OtherActor self false)
    (Utilities|IsValid (Variables|Default|GetWB_TapToGrab)
      (:Is%20Valid
        (Widget|RemovefromParent (Variables|Default|GetWB_TapToGrab))))))

(event OnProjectileStop(ProjectileMovement)
  (params (ImpactResult :type Hit%20Result%20Structure%20%28by%20ref%29))
  ;[0 0 0] OnProjectileStop
  (Transformation|SetActorLocationAndRotation (.impactpoint ImpactResult) (Math|Conversions|RotationFromXVector (.impactnormal ImpactResult)))
  (Variables|Default|SetstickedToWall? true)
  (Collision|SetCollisionObjectType (Variables|Default|GetPipe) "ECC_WorldStatic")
  (Collision|SetCollisionEnabled (Variables|Default|GetGrabBox) "NoCollision"))

(event Custom|SetGrabbedStatus
  (params (isGrabbed? :type Boolean))
  ;[0 0 0] IsGrabbed
  (Variables|Default|SetisGrabbed? isGrabbed?))

(event Custom|isGrabbed
  (params (BP_Player :type Actor%20Object%20Reference))
  ;[0 0 0] IsGrabbed
  (bind _asbp_player (Utilities|Casting|CastToBP_Player BP_Player))
  (if (Pawn|IsLocallyControlled _asbp_player)
    (Utilities|IsValid (Variables|Default|GetWB_TapToGrab)
      (:Is%20Valid
        (Widget|RemovefromParent (Variables|Default|GetWB_TapToGrab))))))

(event EventBeginPlay
  (Collision|SetCollisionEnabled (Variables|Default|GetGrabBox) "QueryAndPhysics"))

(fn ConstructionScript)