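; BP_Armadio is a wardrobe where players choose a power, Super Dash or Super Strength, with doors swung open by a timeline.
; DashPower and StrengthPower flags enable each trigger at BeginPlay.
; Overlapping a trigger disables a local player's input and shows its choice widget if they have no ability.
; Leaving with that ability disables the trigger's collision through server and multicast events; otherwise its DoOnce resets.
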(event OnComponentBeginOverlap(SceltaPotere_Dash)
  (params (OverlappedComponent :type Primitive%20Component%20Object%20Reference) (OtherActor :type Actor%20Object%20Reference) (OtherComp :type Primitive%20Component%20Object%20Reference) (OtherBodyIndex :type Integer) (bFromSweep :type Boolean) (SweepResult :type Hit%20Result%20Structure%20%28by%20ref%29))
  ;[1 1 1] SUper Dash
  (Utilities|FlowControl|DoOnce false
    (:Completed
      (Variables|Default|SetOther%20Actor OtherActor)
      (bind _asbp_player (Utilities|Casting|CastToBP_Player OtherActor))
      (if (Pawn|IsLocallyControlled _asbp_player)
        (if (Utilities|Enum|Equal(Enum) (Variables|/Game/Characters/BP_Player.BP_Player_C|GetAbilityName _asbp_player) (Utilities|Text|MakeLiteralText ""))
          (Input|DisableInput _asbp_player (Pawn|GetLocalViewingPlayerController _asbp_player))
          (Utilities|IsValid (Variables|Default|GetWB_SuperDash)
            (:Is%20Valid
              _)
            (:Is%20Not%20Valid
              (bind _returnvalue (UserInterface|CreateWidget "/Game/Widget/WB_ChooseSuperDash.WB_ChooseSuperDash_C" (Pawn|GetLocalViewingPlayerController _asbp_player)))
              (Variables|Default|SetWB_SuperDash _returnvalue)))
          (UserInterface|Viewport|AddtoViewport (Variables|Default|GetWB_SuperDash) 0)
          (Development|PrintString "Near Armadio"))))))

(event OnComponentEndOverlap(SceltaPotere_Dash)
  (params (OverlappedComponent :type Primitive%20Component%20Object%20Reference) (OtherActor :type Actor%20Object%20Reference) (OtherComp :type Primitive%20Component%20Object%20Reference) (OtherBodyIndex :type Integer))
  (bind _sceltapotere_dash (Variables|Default|GetSceltaPotere_Dash))
  ;[1 1 1] SUper Dash
  (bind _asbp_player (Utilities|Casting|CastToBP_Player OtherActor))
  (if (Utilities|Enum|Equal(Enum) (Variables|/Game/Characters/BP_Player.BP_Player_C|GetAbilityName _asbp_player) (Utilities|Text|MakeLiteralText "Super Dash"))
    (Networking|SwitchHasAuthority
      (:Authority
        (CallFunction|MulticastDisableArmadioDash _sceltapotere_dash))
      (:Remote
        (CallFunction|SrvDisableArmadioDash _sceltapotere_dash)))
    (elif (== (Variables|Default|GetOther%20Actor) OtherActor)
      (CallFunction|ResetDash))))

(event OnComponentBeginOverlap(SceltaPotere_Strength)
  (params (OverlappedComponent :type Primitive%20Component%20Object%20Reference) (OtherActor :type Actor%20Object%20Reference) (OtherComp :type Primitive%20Component%20Object%20Reference) (OtherBodyIndex :type Integer) (bFromSweep :type Boolean) (SweepResult :type Hit%20Result%20Structure%20%28by%20ref%29))
  ;[1 1 1] Super Strength
  (Utilities|FlowControl|DoOnce false
    (:Completed
      (Variables|Default|SetOther%20Actor OtherActor)
      (bind _asbp_player (Utilities|Casting|CastToBP_Player OtherActor))
      (if (Pawn|IsLocallyControlled _asbp_player)
        (if (Utilities|Enum|Equal(Enum) (Variables|/Game/Characters/BP_Player.BP_Player_C|GetAbilityName _asbp_player) (Utilities|Text|MakeLiteralText ""))
          (Input|DisableInput _asbp_player (Pawn|GetLocalViewingPlayerController _asbp_player))
          (Utilities|IsValid (Variables|Default|GetWB_SuperStrength)
            (:Is%20Valid
              _)
            (:Is%20Not%20Valid
              (bind _returnvalue (UserInterface|CreateWidget "/Game/Widget/WB_ChooseSuperStrength.WB_ChooseSuperStrength_C" (Pawn|GetLocalViewingPlayerController _asbp_player)))
              (Variables|Default|SetWB_SuperStrength _returnvalue)))
          (UserInterface|Viewport|AddtoViewport (Variables|Default|GetWB_SuperStrength) 0)
          (Development|PrintString "Near Armadio"))))))

(event OnComponentEndOverlap(SceltaPotere_Strength)
  (params (OverlappedComponent :type Primitive%20Component%20Object%20Reference) (OtherActor :type Actor%20Object%20Reference) (OtherComp :type Primitive%20Component%20Object%20Reference) (OtherBodyIndex :type Integer))
  ;[1 1 1] Super Strength
  (bind _asbp_player (Utilities|Casting|CastToBP_Player OtherActor))
  (if (Utilities|Enum|Equal(Enum) (Variables|/Game/Characters/BP_Player.BP_Player_C|GetAbilityName _asbp_player) (Utilities|Text|MakeLiteralText "Super Strength"))
    (Networking|SwitchHasAuthority
      (:Authority
        (CallFunction|MulticastDisableArmadioStrength))
      (:Remote
        (CallFunction|SrvDisableArmadioStrength)))
    (elif (== (Variables|Default|GetOther%20Actor) OtherActor)
      (CallFunction|ResetStrength))))

(event Custom|OpenArmadio
  (bind _angledoor (Timeline|TimelineOpenArmadio PlayFromStart)
    (:Update
      (Transformation|SetRelativeRotation (Variables|Default|GetAntaSx) (Class|KismetMathLibrary|NegateRotator (Math|Rotator|MakeRotator 0.0 0.0 _angledoor)) false false)
      (Transformation|SetRelativeRotation (Variables|Default|GetAntaDx) (Math|Rotator|MakeRotator 0.0 0.0 _angledoor) false false))))

(event Custom|ResetDash
  ;[1 1 1] SUper Dash
  (Utilities|FlowControl|DoOnce false) ; enters at Reset
)

(event Custom|ResetStrength
  ;[1 1 1] Super Strength
  (Utilities|FlowControl|DoOnce false) ; enters at Reset
)

(event Custom|Multicast_DisableArmadio_Strength
  ;[1 1 1] Super Strength
  (Collision|SetCollisionEnabled (Variables|Default|GetSceltaPotere_Strength) "NoCollision"))

(event Custom|Srv_DisableArmadio_Strength
  ;[1 1 1] Super Strength
  (CallFunction|MulticastDisableArmadioStrength))

(event Custom|Multicast_DisableArmadio_Dash
  (params (Target :type Primitive%20Component%20Object%20Reference))
  ;[1 1 1] SUper Dash
  (Collision|SetCollisionEnabled Target "NoCollision"))

(event Custom|Srv_DisableArmadio_Dash
  (params (Target :type Primitive%20Component%20Object%20Reference))
  ;[1 1 1] SUper Dash
  (CallFunction|MulticastDisableArmadioDash Target))

(event EventBeginPlay
  (if (Variables|Default|GetDashPower)
    (Collision|SetCollisionEnabled (Variables|Default|GetSceltaPotere_Dash) "QueryAndPhysics")
    (else
      (Collision|SetCollisionEnabled (Variables|Default|GetSceltaPotere_Dash) "NoCollision")))
  (if (Variables|Default|GetStrengthPower)
    (Collision|SetCollisionEnabled (Variables|Default|GetSceltaPotere_Strength) "QueryAndPhysics")
    (else
      (Collision|SetCollisionEnabled (Variables|Default|GetSceltaPotere_Strength) "NoCollision"))))

(event Collision|EventActorBeginOverlap
  (params (OtherActor :type Actor%20Object%20Reference)))

(event EventTick
  (params (DeltaSeconds :type Float%20%28single-precision%29)))

(fn ConstructionScript)