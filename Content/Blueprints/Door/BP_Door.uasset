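; BP_Door is an interactable door that prompts a nearby player and swings open.
; An overlap box messages the locally controlled BP_Player whether it is near the door, passing the door as target.
; While the door is closed, entering also shows a cached tap-to-interact widget, which leaving removes.
; OpenDoor, not called within this Blueprint, disables door collision, sets IsOpen and rotates the door's yaw through a timeline.
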(event OnComponentBeginOverlap(CollionBoxOpen)
  (params (OverlappedComponent :type Primitive%20Component%20Object%20Reference) (OtherActor :type Actor%20Object%20Reference) (OtherComp :type Primitive%20Component%20Object%20Reference) (OtherBodyIndex :type Integer) (bFromSweep :type Boolean) (SweepResult :type Hit%20Result%20Structure%20%28by%20ref%29))
  (bind _asbp_player (Utilities|Casting|CastToBP_Player OtherActor))
  (if (Pawn|IsLocallyControlled _asbp_player)
    (if (not (Variables|Default|GetisOpen?))
      (Class|BPIDoor|IsNearDoor(Message) OtherActor self true)
      (Utilities|IsValid (Variables|Default|GetWB_TapToInteract)
        (:Is%20Valid
          _)
        (:Is%20Not%20Valid
          (bind _returnvalue (UserInterface|CreateWidget "/Game/Widget/WB_TapEToInteract.WB_TapEToInteract_C" (Pawn|GetLocalViewingPlayerController _asbp_player)))
          (Variables|Default|SetWB_TapToInteract _returnvalue)))
      (UserInterface|Viewport|AddtoViewport (Variables|Default|GetWB_TapToInteract) 0)
      (Development|PrintString "Near Door"))))

(event OnComponentEndOverlap(CollionBoxOpen)
  (params (OverlappedComponent :type Primitive%20Component%20Object%20Reference) (OtherActor :type Actor%20Object%20Reference) (OtherComp :type Primitive%20Component%20Object%20Reference) (OtherBodyIndex :type Integer))
  (bind _asbp_player (Utilities|Casting|CastToBP_Player OtherActor))
  (if (Pawn|IsLocallyControlled _asbp_player)
    (Class|BPIDoor|IsNearDoor(Message) OtherActor self false)
    (Utilities|IsValid (Variables|Default|GetWB_TapToInteract)
      (:Is%20Valid
        (Widget|RemovefromParent (Variables|Default|GetWB_TapToInteract))
        (Development|PrintString "Not Near Door")))))

(event Custom|OpenDoor
  (Collision|SetCollisionEnabled (Variables|Default|GetDoor) "NoCollision")
  (Variables|Default|SetisOpen? true)
  (bind _angle (Timeline|OpenDoorTimeline PlayFromStart)
    (:Update
      (Transformation|SetRelativeRotation (Variables|Default|GetDoor) (Math|Rotator|MakeRotator 0.0 0.0 _angle) false false))))

(event EventBeginPlay)

(event Collision|EventActorBeginOverlap
  (params (OtherActor :type Actor%20Object%20Reference)))

(event EventTick
  (params (DeltaSeconds :type Float%20%28single-precision%29)))

(fn ConstructionScript)