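; BP_Map is an inn map actor that signals when the local player is close enough to interact with it.
; Its Box overlap events filter for a locally controlled BP_Player_Inn and send it IsNearMapMessage, true on entry and false on exit.
; A tap-to-interact widget is created on first use, cached, and added to or removed from the viewport, with a debug print on entry.
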(event OnComponentBeginOverlap(Box)
  (params (OverlappedComponent :type Primitive%20Component%20Object%20Reference) (OtherActor :type Actor%20Object%20Reference) (OtherComp :type Primitive%20Component%20Object%20Reference) (OtherBodyIndex :type Integer) (bFromSweep :type Boolean) (SweepResult :type Hit%20Result%20Structure%20%28by%20ref%29))
  (bind _asbp_player_inn (Utilities|Casting|CastToBP_Player_Inn OtherActor))
  (if (Pawn|IsLocallyControlled _asbp_player_inn)
    (Class|BPIMap|IsNearMap(Message) OtherActor true)
    (Utilities|IsValid (Variables|Default|GetWB_TapToInteract)
      (:Is%20Valid
        _)
      (:Is%20Not%20Valid
        (bind _returnvalue (UserInterface|CreateWidget "/Game/Widget/WB_TapEToInteract.WB_TapEToInteract_C" (Pawn|GetLocalViewingPlayerController _asbp_player_inn)))
        (Variables|Default|SetWB_TapToInteract _returnvalue)))
    (UserInterface|Viewport|AddtoViewport (Variables|Default|GetWB_TapToInteract) 0)
    (Development|PrintString "NearMap")))

(event OnComponentEndOverlap(Box)
  (params (OverlappedComponent :type Primitive%20Component%20Object%20Reference) (OtherActor :type Actor%20Object%20Reference) (OtherComp :type Primitive%20Component%20Object%20Reference) (OtherBodyIndex :type Integer))
  (bind _asbp_player_inn (Utilities|Casting|CastToBP_Player_Inn OtherActor))
  (if (Pawn|IsLocallyControlled _asbp_player_inn)
    (Class|BPIMap|IsNearMap(Message) OtherActor false)
    (Utilities|IsValid (Variables|Default|GetWB_TapToInteract)
      (:Is%20Valid
        (Widget|RemovefromParent (Variables|Default|GetWB_TapToInteract))))))

(event EventBeginPlay)

(event Collision|EventActorBeginOverlap
  (params (OtherActor :type Actor%20Object%20Reference)))

(event EventTick
  (params (DeltaSeconds :type Float%20%28single-precision%29)))

(fn ConstructionScript)