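; Interactable book actor for the Inn that shows an interact prompt when the player comes near.
; Box overlap events act only for a locally controlled BP_Player_Inn, notifying it through IsNearBookMessage when it enters or leaves.
; The WB_TapEToInteract widget is created on first overlap, cached for reuse, added to the viewport on entry and removed on exit.
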(event OnComponentBeginOverlap(Box)
  (params (OverlappedComponent :type Primitive%20Component%20Object%20Reference) (OtherActor :type Actor%20Object%20Reference) (OtherComp :type Primitive%20Component%20Object%20Reference) (OtherBodyIndex :type Integer) (bFromSweep :type Boolean) (SweepResult :type Hit%20Result%20Structure%20%28by%20ref%29))
  (bind _asbp_player_inn (Utilities|Casting|CastToBP_Player_Inn OtherActor))
  (if (Pawn|IsLocallyControlled _asbp_player_inn)
    (Class|BPINPCBook|IsNearBook(Message) OtherActor true)
    (Utilities|IsValid (Variables|Default|GetWB%20Tap%20To%20Interact)
      (:Is%20Valid
        _)
      (:Is%20Not%20Valid
        (bind _returnvalue (UserInterface|CreateWidget "/Game/Widget/WB_TapEToInteract.WB_TapEToInteract_C" (Pawn|GetLocalViewingPlayerController _asbp_player_inn)))
        (Variables|Default|SetWB%20Tap%20To%20Interact _returnvalue)))
    (UserInterface|Viewport|AddtoViewport (Variables|Default|GetWB%20Tap%20To%20Interact) 0)))

(event OnComponentEndOverlap(Box)
  (params (OverlappedComponent :type Primitive%20Component%20Object%20Reference) (OtherActor :type Actor%20Object%20Reference) (OtherComp :type Primitive%20Component%20Object%20Reference) (OtherBodyIndex :type Integer))
  (bind _asbp_player_inn (Utilities|Casting|CastToBP_Player_Inn OtherActor))
  (if (Pawn|IsLocallyControlled _asbp_player_inn)
    (Class|BPINPCBook|IsNearBook(Message) OtherActor false)
    (Utilities|IsValid (Variables|Default|GetWB%20Tap%20To%20Interact)
      (:Is%20Valid
        (Widget|RemovefromParent (Variables|Default|GetWB%20Tap%20To%20Interact))))))

(event EventBeginPlay)

(event Collision|EventActorBeginOverlap
  (params (OtherActor :type Actor%20Object%20Reference)))

(event EventTick
  (params (DeltaSeconds :type Float%20%28single-precision%29)))

(fn ConstructionScript)