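; BP_StartLevelPoint is a trigger point on the game map that marks the entry to Zone3_Level1.
; Box overlaps react only to a locally controlled BP_Player_GameMap, which receives IsNearLevelMessage with the hardcoded level name on entry and a cleared one on exit.
; The WB_StartLevel widget is created on first entry, cached, then shown and removed as the player enters and leaves.
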(event OnComponentBeginOverlap(Box)
  (params (OverlappedComponent :type Primitive%20Component%20Object%20Reference) (OtherActor :type Actor%20Object%20Reference) (OtherComp :type Primitive%20Component%20Object%20Reference) (OtherBodyIndex :type Integer) (bFromSweep :type Boolean) (SweepResult :type Hit%20Result%20Structure%20%28by%20ref%29))
  (bind _asbp_player_game_map (Utilities|Casting|CastToBP_Player_GameMap OtherActor))
  (if (Pawn|IsLocallyControlled _asbp_player_game_map)
    (Class|BPIIconLevel|IsNearLevel(Message) OtherActor true "Zone3_Level1")
    (Utilities|IsValid (Variables|Default|GetWB_StartLevel)
      (:Is%20Valid
        _)
      (:Is%20Not%20Valid
        (bind _returnvalue (UserInterface|CreateWidget "/Game/Widget/WB_StartLevel.WB_StartLevel_C" (Pawn|GetLocalViewingPlayerController _asbp_player_game_map)))
        (Variables|Default|SetWB_StartLevel _returnvalue)))
    (UserInterface|Viewport|AddtoViewport (Variables|Default|GetWB_StartLevel) 0)))

(event OnComponentEndOverlap(Box)
  (params (OverlappedComponent :type Primitive%20Component%20Object%20Reference) (OtherActor :type Actor%20Object%20Reference) (OtherComp :type Primitive%20Component%20Object%20Reference) (OtherBodyIndex :type Integer))
  (bind _wb_startlevel (Variables|Default|GetWB_StartLevel))
  (bind _asbp_player_game_map (Utilities|Casting|CastToBP_Player_GameMap OtherActor))
  (if (Pawn|IsLocallyControlled _asbp_player_game_map)
    (Class|BPIIconLevel|IsNearLevel(Message) OtherActor false)
    (Utilities|IsValid _wb_startlevel
      (:Is%20Valid
        (Widget|RemovefromParent _wb_startlevel)))))

(fn ConstructionScript)