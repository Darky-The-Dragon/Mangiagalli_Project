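; BP_LeverDoubleDoor is an interactable lever, apparently for a double door, that players can use when standing near it.
; Box overlaps tell the locally controlled BP_Player via a message that it is near the lever, and show or remove a cached tap-to-interact widget.
; UseLever and UseLeverReverse play the LevelAnim sequence forward or backward through a newly created player, while DeactivateLever disables the box's collision.
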(event OnComponentBeginOverlap(Box)
  (params (OverlappedComponent :type Primitive%20Component%20Object%20Reference) (OtherActor :type Actor%20Object%20Reference) (OtherComp :type Primitive%20Component%20Object%20Reference) (OtherBodyIndex :type Integer) (bFromSweep :type Boolean) (SweepResult :type Hit%20Result%20Structure%20%28by%20ref%29))
  (bind _asbp_player (Utilities|Casting|CastToBP_Player OtherActor))
  (if (Pawn|IsLocallyControlled _asbp_player)
    (Class|BPILever|IsNearLeverDoubleDoor(Message) OtherActor self true true)
    (Utilities|IsValid (Variables|Default|GetWB_TapToInteract)
      (:Is%20Valid
        _)
      (:Is%20Not%20Valid
        (bind _returnvalue (UserInterface|CreateWidget "/Game/Widget/WB_TapEToInteract.WB_TapEToInteract_C" (Pawn|GetLocalViewingPlayerController _asbp_player)))
        (Variables|Default|SetWB_TapToInteract _returnvalue)))
    (UserInterface|Viewport|AddtoViewport (Variables|Default|GetWB_TapToInteract) 0)
    (Development|PrintString "Near DoubleDoor")))

(event OnComponentEndOverlap(Box)
  (params (OverlappedComponent :type Primitive%20Component%20Object%20Reference) (OtherActor :type Actor%20Object%20Reference) (OtherComp :type Primitive%20Component%20Object%20Reference) (OtherBodyIndex :type Integer))
  (bind _asbp_player (Utilities|Casting|CastToBP_Player OtherActor))
  (if (Pawn|IsLocallyControlled _asbp_player)
    (Class|BPILever|IsNearLeverDoubleDoor(Message) OtherActor self false false)
    (Utilities|IsValid (Variables|Default|GetWB_TapToInteract)
      (:Is%20Valid
        (Widget|RemovefromParent (Variables|Default|GetWB_TapToInteract))
        (Development|PrintString "Not near DoubleDoor")))))

(event Custom|DeactivateLever
  (Collision|SetCollisionEnabled (Variables|Default|GetBox) "NoCollision"))

(event Custom|UseLever
  (bind _outactor (Sequencer|Player|CreateLevelSequencePlayer (Variables|Default|GetLevelAnim)))
  (Sequencer|Player|Play (Variables|/Script/LevelSequence.LevelSequenceActor|GetSequencePlayer _outactor) :!class /Script/MovieScene.MovieSceneSequencePlayer))

(event Custom|UseLeverReverse
  (bind _outactor (Sequencer|Player|CreateLevelSequencePlayer (Variables|Default|GetLevelAnim)))
  (Class|MovieSceneSequencePlayer|PlayReverse (Variables|/Script/LevelSequence.LevelSequenceActor|GetSequencePlayer _outactor)))

(event EventBeginPlay)

(event Collision|EventActorBeginOverlap
  (params (OtherActor :type Actor%20Object%20Reference)))

(event EventTick
  (params (DeltaSeconds :type Float%20%28single-precision%29)))

(fn ConstructionScript)