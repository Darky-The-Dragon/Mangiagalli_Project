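; BP_StartCutscene is a box trigger that starts Level Sequence cutscenes when BP_Player overlaps it.
; A DoOnce precedes the player cast, so the first overlap by any actor uses up the trigger.
; It plays all NonLoopAnim sequences at once, or starts LoopAnim sequences looping if that array is empty.
; Each one-shot's OnStop also starts the loops, so several one-shots create duplicate looping players.
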(event OnComponentBeginOverlap(Box)
  (params (OverlappedComponent :type Primitive%20Component%20Object%20Reference) (OtherActor :type Actor%20Object%20Reference) (OtherComp :type Primitive%20Component%20Object%20Reference) (OtherBodyIndex :type Integer) (bFromSweep :type Boolean) (SweepResult :type Hit%20Result%20Structure%20%28by%20ref%29))
  (Utilities|FlowControl|DoOnce false
    (:Completed
      (Development|PrintString "StartCutscene")
      (bind _asbp_player (Utilities|Casting|CastToBP_Player OtherActor))
      (if (!= (Utilities|Array|Length (Variables|Default|GetNonLoopAnim)) 0)
        (for _array_element (Variables|Default|GetNonLoopAnim)
          (Utilities|IsValid _array_element
            (:Is%20Valid
              (bind _outactor (Sequencer|Player|CreateLevelSequencePlayer _array_element))
              (Sequencer|Player|Play (Variables|/Script/LevelSequence.LevelSequenceActor|GetSequencePlayer _outactor) :!class /Script/MovieScene.MovieSceneSequencePlayer)
              (EventDispatchers|AssignOnStop (Variables|/Script/LevelSequence.LevelSequenceActor|GetSequencePlayer _outactor) (delegate Custom|OnStop_Event)))))
        (else
          (for _array_element_2 (Variables|Default|GetLoopAnim)
            (Utilities|IsValid _array_element_2
              (:Is%20Valid
                (bind _outactor_2 (Sequencer|Player|CreateLevelSequencePlayer _array_element_2))
                (Class|MovieSceneSequencePlayer|PlayLooping (Variables|/Script/LevelSequence.LevelSequenceActor|GetSequencePlayer _outactor_2) -1)))))))))

(event Custom|OnStop_Event
  (for _array_element (Variables|Default|GetLoopAnim)
    (Utilities|IsValid _array_element
      (:Is%20Valid
        (bind _outactor (Sequencer|Player|CreateLevelSequencePlayer _array_element))
        (Class|MovieSceneSequencePlayer|PlayLooping (Variables|/Script/LevelSequence.LevelSequenceActor|GetSequencePlayer _outactor) -1)))))

(event EventBeginPlay)

(event Collision|EventActorBeginOverlap
  (params (OtherActor :type Actor%20Object%20Reference)))

(event EventTick
  (params (DeltaSeconds :type Float%20%28single-precision%29)))

(fn ConstructionScript)