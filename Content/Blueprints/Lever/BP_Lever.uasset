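; BP_Lever is an interactable lever that triggers level sequence animations when used.
; Its box overlap shows a tap-E prompt widget to the locally controlled BP_Player and removes it on exit.
; UseLever, which has no caller in this Blueprint, plays the lever sequence.
; When that sequence stops, it starts every valid NonLoopAnim sequence once and every LoopAnim sequence on endless loop, all simultaneously.
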(event OnComponentBeginOverlap(Box)
  (params (OverlappedComponent :type Primitive%20Component%20Object%20Reference) (OtherActor :type Actor%20Object%20Reference) (OtherComp :type Primitive%20Component%20Object%20Reference) (OtherBodyIndex :type Integer) (bFromSweep :type Boolean) (SweepResult :type Hit%20Result%20Structure%20%28by%20ref%29))
  (bind _asbp_player (Utilities|Casting|CastToBP_Player OtherActor))
  (if (Pawn|IsLocallyControlled _asbp_player)
    (Utilities|IsValid (Variables|Default|GetWB_TapToInteract)
      (:Is%20Valid
        _)
      (:Is%20Not%20Valid
        (bind _returnvalue (UserInterface|CreateWidget "/Game/Widget/WB_TapEToInteract.WB_TapEToInteract_C"))
        (Variables|Default|SetWB_TapToInteract _returnvalue)))
    (UserInterface|Viewport|AddtoViewport (Variables|Default|GetWB_TapToInteract) 0)))

(event OnComponentEndOverlap(Box)
  (params (OverlappedComponent :type Primitive%20Component%20Object%20Reference) (OtherActor :type Actor%20Object%20Reference) (OtherComp :type Primitive%20Component%20Object%20Reference) (OtherBodyIndex :type Integer))
  (bind _asbp_player (Utilities|Casting|CastToBP_Player OtherActor))
  (if (Pawn|IsLocallyControlled _asbp_player)
    (Utilities|IsValid (Variables|Default|GetWB_TapToInteract)
      (:Is%20Valid
        (Widget|RemovefromParent (Variables|Default|GetWB_TapToInteract))))))

(event Custom|OnStop_Event
  (for _array_element (Variables|Default|GetNonLoopAnim)
    (Utilities|IsValid _array_element
      (:Is%20Valid
        (bind _outactor (Sequencer|Player|CreateLevelSequencePlayer _array_element))
        (Sequencer|Player|Play (Variables|/Script/LevelSequence.LevelSequenceActor|GetSequencePlayer _outactor) :!class /Script/MovieScene.MovieSceneSequencePlayer))))
  (for _array_element_2 (Variables|Default|GetLoopAnim)
    (Utilities|IsValid _array_element_2
      (:Is%20Valid
        (bind _outactor_2 (Sequencer|Player|CreateLevelSequencePlayer _array_element_2))
        (Class|MovieSceneSequencePlayer|PlayLooping (Variables|/Script/LevelSequence.LevelSequenceActor|GetSequencePlayer _outactor_2) -1)))))

(event Custom|UseLever
  (bind _outactor (Sequencer|Player|CreateLevelSequencePlayer (Variables|Default|GetLevelAnim)))
  (Sequencer|Player|Play (Variables|/Script/LevelSequence.LevelSequenceActor|GetSequencePlayer _outactor) :!class /Script/MovieScene.MovieSceneSequencePlayer)
  (EventDispatchers|AssignOnStop (Variables|/Script/LevelSequence.LevelSequenceActor|GetSequencePlayer _outactor) (delegate Custom|OnStop_Event)))

(event EventBeginPlay)

(event Collision|EventActorBeginOverlap
  (params (OtherActor :type Actor%20Object%20Reference)))

(event EventTick
  (params (DeltaSeconds :type Float%20%28single-precision%29)))

(fn ConstructionScript)