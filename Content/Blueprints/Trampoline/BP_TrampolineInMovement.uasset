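; BP_TrampolineInMovement is a trampoline actor that tells a player when they enter or leave its jump zone.
; Begin and end overlaps on its ReadyTrampoline component filter for a locally controlled BP_Player, then send IsInTrampolineMessage with true or false and print a debug string.
; The Blueprint contains no launch or movement logic; it only signals the zone state to the player.
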(event OnComponentBeginOverlap(ReadyTrampoline)
  (params (OverlappedComponent :type Primitive%20Component%20Object%20Reference) (OtherActor :type Actor%20Object%20Reference) (OtherComp :type Primitive%20Component%20Object%20Reference) (OtherBodyIndex :type Integer) (bFromSweep :type Boolean) (SweepResult :type Hit%20Result%20Structure%20%28by%20ref%29))
  (bind _asbp_player (Utilities|Casting|CastToBP_Player OtherActor))
  (if (Pawn|IsLocallyControlled _asbp_player)
    (Class|BPITrampoline|IsinTrampoline(Message) OtherActor true)
    (Development|PrintString "Can Jump Trampoline Movement" true true "(R=0.000000,G=0.660000,B=1.000000,A=1.000000)" 5.0)))

(event OnComponentEndOverlap(ReadyTrampoline)
  (params (OverlappedComponent :type Primitive%20Component%20Object%20Reference) (OtherActor :type Actor%20Object%20Reference) (OtherComp :type Primitive%20Component%20Object%20Reference) (OtherBodyIndex :type Integer))
  (bind _asbp_player (Utilities|Casting|CastToBP_Player OtherActor))
  (if (Pawn|IsLocallyControlled _asbp_player)
    (Class|BPITrampoline|IsinTrampoline(Message) OtherActor false)
    (Development|PrintString "Outside  Trampoline in Movement" true true "(R=0.000000,G=0.660000,B=1.000000,A=1.000000)" 5.0)))

(event EventBeginPlay)

(fn ConstructionScript)