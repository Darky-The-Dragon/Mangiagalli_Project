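; Climbable ladder actor that tells the player character when it can interact with the ladder and when to leave it.
; EnterBox overlaps send the interaction message on entry and exit; entry also disables DownLadder collision and enables ExitBox.
; ExitBox overlap sends the exit message with two WarpLocation points as exit targets, then restores DownLadder collision.
; All overlap handling responds only to player character 0.
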(event OnComponentBeginOverlap(ExitBox)
  (params (OverlappedComponent :type Primitive%20Component%20Object%20Reference) (OtherActor :type Actor%20Object%20Reference) (OtherComp :type Primitive%20Component%20Object%20Reference) (OtherBodyIndex :type Integer) (bFromSweep :type Boolean) (SweepResult :type Hit%20Result%20Structure%20%28by%20ref%29))
  ;[1 1 1] On exit box entered
  (if (== OtherActor (Game|GetPlayerCharacter 0))
    (Class|LadderBPI|ExitLadder(Message) OtherActor (- (Transformation|GetWorldLocation (Variables|Default|GetWarpLocationForExit)) "0.000000,0.000000,0.000000") (- (Transformation|GetWorldLocation (Variables|Default|GetWarpLocationForExit1)) "0.000000,0.000000,0.000000"))
    (Collision|SetCollisionEnabled (Variables|Default|GetDownLadder) "QueryAndPhysics")))

(event OnComponentBeginOverlap(EnterBox)
  (params (OverlappedComponent :type Primitive%20Component%20Object%20Reference) (OtherActor :type Actor%20Object%20Reference) (OtherComp :type Primitive%20Component%20Object%20Reference) (OtherBodyIndex :type Integer) (bFromSweep :type Boolean) (SweepResult :type Hit%20Result%20Structure%20%28by%20ref%29))
  ;[1 1 1] Can interact with ladder if entered the box
  (if (== OtherActor (Game|GetPlayerCharacter 0))
    (Class|LadderBPI|SetLadderInteraction(Message) OtherActor self true)
    (Collision|SetCollisionEnabled (Variables|Default|GetDownLadder) "NoCollision")
    (Collision|SetCollisionEnabled (Variables|Default|GetExitBox) "QueryAndPhysics")))

(event OnComponentEndOverlap(EnterBox)
  (params (OverlappedComponent :type Primitive%20Component%20Object%20Reference) (OtherActor :type Actor%20Object%20Reference) (OtherComp :type Primitive%20Component%20Object%20Reference) (OtherBodyIndex :type Integer))
  (if (== OtherActor (Game|GetPlayerCharacter 0))
    (Class|LadderBPI|SetLadderInteraction(Message) OtherActor self false)))

(fn ConstructionScript)