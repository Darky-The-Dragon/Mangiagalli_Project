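; Game mode for the Inn map that tracks connected player controllers and spawns players at numbered PlayerStarts.
; Each new player updates the expected count from the game instance; solo spawns at start "0", while multiplayer respawns all tracked players by index, delaying briefly only when all have connected.
; LevelStart then re-enables everyone's input after a short delay.
; DisableAllInput disables input for all controllers, and logout removes the leaving one.
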(event Custom|LevelStart
  ;[1 1 1] LevelStart. Fa partire il countDown per ogni giocatore, ed alla fine di esso riattiva l'input per tutti
  (Utilities|FlowControl|Delay 0.2)
  (for _array_element (Variables|Default|GetAll_ConnectedControllers)
    (Default|EnableAllInput _array_element)))

(event Custom|DisableAllInput
  (for _array_element (Variables|Default|GetAll_ConnectedControllers)
    (Input|DisableInput _array_element)))

(event EventOnLogout
  (params (ExitingController :type Controller%20Object%20Reference))
  (bind _asbp_player_controller_inn (Utilities|Casting|CastToBP_PlayerController_Inn ExitingController))
  (Utilities|Array|RemoveItem (Variables|Default|GetAll_ConnectedControllers) _asbp_player_controller_inn)
  (Math|Integer|DecrementInt (Variables|Default|GetNum_ExpectedPlayers)))

(event EventHandleStartingNewPlayer
  (params (NewPlayer :type Player%20Controller%20Object%20Reference))
  ;[1 1 1] HandleStartingNewPlayer. Gestisce la connessione di un nuovo giocatore, facendolo spawnare nel punto giusto
  (bind _asbp_player_controller_inn (Utilities|Casting|CastToBP_PlayerController_Inn NewPlayer))
  (Utilities|Array|Add (Variables|Default|GetAll_ConnectedControllers) _asbp_player_controller_inn)
  (bind _asbp_game_instance (Utilities|Casting|CastToBP_GameInstance (Game|GetGameInstance)))
  (Variables|Default|SetNum_ExpectedPlayers (Variables|/Game/Blueprints/FrameWork/BP_GameInstance.BP_GameInstance_C|GetNum%20Connected%20Player _asbp_game_instance))
  (if (Variables|/Game/Blueprints/FrameWork/BP_GameInstance.BP_GameInstance_C|GetinSoloGame _asbp_game_instance)
    (Variables|Default|SetNum_ExpectedPlayers 1)
    (Class|GameModeBase|RestartPlayeratPlayerStart (Utilities|Array|Get(acopy) (Variables|Default|GetAll_ConnectedControllers)) (Class|GameModeBase|FindPlayerStart 0 "0"))
    (CallFunction|LevelStart)
    (else
      (if (== (Variables|Default|GetNum_ExpectedPlayers) (Utilities|Array|Length (Variables|Default|GetAll_ConnectedControllers)))
        (Utilities|FlowControl|Delay 0.5)
        (else
          ;;[1 0 0] Fast testing animation
          (Development|PrintString "PIE launch enabled")))
      (for (_array_element _array_index) (Variables|Default|GetAll_ConnectedControllers)
        (Class|GameModeBase|RestartPlayeratPlayerStart _array_element (Class|GameModeBase|FindPlayerStart _array_element (Utilities|String|ToString(Integer) _array_index))))
      (CallFunction|LevelStart))))

(fn ConstructionScript)