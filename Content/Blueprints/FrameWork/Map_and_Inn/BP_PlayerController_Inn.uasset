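; Player controller for the Inn level that sets up local input and drives in-game HUD and loading-screen widgets.
; On BeginPlay the local controller adds the Enhanced Input context, clears widgets and switches to game-only input.
; Events toggle pawn input, reveal the HUD, start the countdown, show the load screen, or end the client session back to the main menu.
; A helper loads or creates the saved player profile, though nothing here calls it.
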(event Custom|EndClientSession
  ;[0 0 0] End Client Session
  (bind _asbp_game_instance (Utilities|Casting|CastToBP_GameInstance (Game|GetGameInstance)))
  (Variables|/Game/Blueprints/FrameWork/BP_GameInstance.BP_GameInstance_C|SetMP_isPauseMenuVisible _asbp_game_instance false)
  (|DestroySession self
    (:then
      (Game|OpenLevel(byName) "MainMenuMap"))))

(event Custom|GameStartCountdown
  (Default|GameStartCountDown (Variables|Default|GetWB_IngameHUD)))

(event Custom|CreateLoadScreen
  ;[1 1 1] Create Load Screen
  (CallFunction|UIShowLoadScreen))

(event Custom|EnableAllInput
  (Input|EnableInput (Pawn|GetControlledPawn) self))

(event Custom|DisableAllInput
  (Input|DisableInput (Pawn|GetControlledPawn) self))

(event Custom|UnHide_IngameHUD
  ;[0 0 0] Unhide Ingame HUD
  (Widget|SetVisibility (Variables|Default|GetWB_IngameHUD) "Visible"))

(event EventBeginPlay
  (if (Pawn|IsLocalPlayerController)
    ;[1 1 1] Attivazione del sistema avanzato di gestione dell'input
    (Input|AddMappingContext (PlayerController|LocalPlayerSubsystems|GetEnhancedInputLocalPlayerSubsystem) "/Game/Input/IMC_Input.IMC_Input" 0 "(bIgnoreAllPressedKeysUntilRelease=True,bForceImmediately=False,bNotifyUserSettings=False)")
    (Viewport|RemoveAllWidgets)
    (Input|SetInputModeGameOnly self false)
    (Variables|Default|SetbShowMouseCursor false)))

(fn ConstructionScript)

(fn UIShowinGameHUD
  (Utilities|IsValid (Variables|Default|GetWB_IngameHUD)
    (:Is%20Valid
      _)
    (:Is%20Not%20Valid
      (bind _returnvalue (UserInterface|CreateWidget "/Game/Widget/WB_InagameHUD.WB_InagameHUD_C" self))
      (Variables|Default|SetWB_IngameHUD _returnvalue)))
  (UserInterface|Viewport|AddtoViewport (Variables|Default|GetWB_IngameHUD) 0)
  (return))

(fn UIShowLoadScreen
  (Viewport|RemoveAllWidgets)
  (Utilities|IsValid (Variables|Default|GetWB_LoadScreen)
    (:Is%20Valid
      _)
    (:Is%20Not%20Valid
      (bind _returnvalue (UserInterface|CreateWidget "/Game/Widget/WB_LoadScreen.WB_LoadScreen_C" self))
      (Variables|Default|SetWB_LoadScreen _returnvalue)))
  (UserInterface|Viewport|AddtoViewport (Variables|Default|GetWB_LoadScreen) 0)
  (return))

(fn LoadSavedProfile
  (bind _returnvalue (SaveGame|DoesSaveGameExist "PlayerProfile_Slot"))
  (if _returnvalue
    _
    (else
      (bind _returnvalue_2 (SaveGame|CreateSaveGameObject "/Game/SavedData/SG_PlayerProfile.SG_PlayerProfile_C"))
      (SaveGame|SaveGametoSlot _returnvalue_2 "PlayerProfile_Slot")))
  (bind _returnvalue_3 (SaveGame|LoadGamefromSlot "PlayerProfile_Slot"))
  (bind _assg_player_profile (Utilities|Casting|CastToSG_PlayerProfile _returnvalue_3))
  (Variables|Default|SetPlayerProfileInfo (Variables|/Game/SavedData/SG_PlayerProfile.SG_PlayerProfile_C|GetPlayerProfile _assg_player_profile))
  (return))