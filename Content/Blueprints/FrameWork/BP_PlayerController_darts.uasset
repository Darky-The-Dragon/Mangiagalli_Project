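; Player controller for the darts minigame that sets up input and the in-game HUD for the local player.
; On BeginPlay it adds the Enhanced Input mapping context, clears widgets, creates or reuses the darts minigame widget with its title spawn, and switches to game-only input.
; Events re-enable pawn input, unhide the HUD, and end a client session by clearing the pause-menu flag, destroying the session and loading the main menu.
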(event Custom|EndClientSession
  ;[0 0 0] End Client Session
  (bind _asbp_game_instance (Utilities|Casting|CastToBP_GameInstance (Game|GetGameInstance)))
  (Variables|/Game/Blueprints/FrameWork/BP_GameInstance.BP_GameInstance_C|SetMP_isPauseMenuVisible _asbp_game_instance false)
  (|DestroySession self
    (:then
      (Game|OpenLevel(byName) "MainMenuMap"))))

(event Custom|UnHide_IngameHUD
  ;[0 0 0] Unhide Ingame HUD
  (Widget|SetVisibility (Variables|Default|GetWB_IngameHUD) "Visible"))

(event Custom|EnableAllInput
  (Input|EnableInput (Pawn|GetControlledPawn) self))

(event EventBeginPlay
  (if (Pawn|IsLocalPlayerController)
    ;[1 1 1] Attivazione del sistema avanzato di gestione dell'input
    (Input|AddMappingContext (PlayerController|LocalPlayerSubsystems|GetEnhancedInputLocalPlayerSubsystem) "/Game/Input/IMC_Input.IMC_Input" 0 "(bIgnoreAllPressedKeysUntilRelease=True,bForceImmediately=False,bNotifyUserSettings=False)")
    (Viewport|RemoveAllWidgets)
    (CallFunction|UIShowinGameHUD)
    (Input|SetInputModeGameOnly self false)
    (Variables|Default|SetbShowMouseCursor false)))

(fn ConstructionScript)

(fn UIShowinGameHUD
  (Utilities|IsValid (Variables|Default|GetWB_IngameHUD)
    (:Is%20Valid
      _)
    (:Is%20Not%20Valid
      (bind _returnvalue (UserInterface|CreateWidget "/Game/Blueprints/Darts/WB_DartsMinigame.WB_DartsMinigame_C" self))
      (Variables|Default|SetWB_IngameHUD _returnvalue)))
  (UserInterface|Viewport|AddtoViewport (Variables|Default|GetWB_IngameHUD) 0)
  (Default|TitleSpawning (Variables|Default|GetWB_IngameHUD))
  (return))