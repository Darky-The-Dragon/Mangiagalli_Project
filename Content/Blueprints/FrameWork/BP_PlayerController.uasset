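; Player controller for a multiplayer game, handling local input setup, in-game UI and leaving a session.
; On BeginPlay the local controller adds the Enhanced Input mapping context, clears widgets, shows the HUD and switches to game-only input.
; Events toggle pawn input, unhide the HUD, start its countdown and briefly show lazily created, cached single or group death ("caught") screens.
; Ending a client session resets the GameInstance pause flag, destroys the session and opens the main menu.
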(event Custom|EndClientSession
  ;[0 0 0] End Client Session
  (bind _asbp_game_instance (Utilities|Casting|CastToBP_GameInstance (Game|GetGameInstance)))
  (Variables|/Game/Blueprints/FrameWork/BP_GameInstance.BP_GameInstance_C|SetMP_isPauseMenuVisible _asbp_game_instance false)
  (|DestroySession self
    (:then
      (Game|OpenLevel(byName) "MainMenuMap"))))

(event Custom|GameStartCountdown
  (Default|GameStartCountDown (Variables|Default|GetWB_IngameHUD)))

(event Custom|UnHide_IngameHUD
  ;[0 0 0] Unhide Ingame HUD
  (Widget|SetVisibility (Variables|Default|GetWB_IngameHUD) "Visible"))

(event Custom|EnableAllInput
  (Input|EnableInput (Pawn|GetControlledPawn) self))

(event Custom|DisableAllInput
  (Input|DisableInput (Pawn|GetControlledPawn) self))

(event Custom|UI_ShowInGameDeath_Single
  (Utilities|IsValid (Variables|Default|GetWB_UI_Death_Single)
    (:Is%20Valid
      _)
    (:Is%20Not%20Valid
      (bind _returnvalue (UserInterface|CreateWidget "/Game/Widget/WB_Beccato.WB_Beccato_C" self))
      (Variables|Default|SetWB_UI_Death_Single _returnvalue)))
  (UserInterface|Viewport|AddtoViewport (Variables|Default|GetWB_UI_Death_Single) 0)
  (Utilities|FlowControl|Delay 3.0)
  (Widget|RemovefromParent (Variables|Default|GetWB_UI_Death_Single)))

(event Custom|UI_ShowInGameDeath_All
  (Utilities|IsValid (Variables|Default|GetWB_UI_Death_All)
    (:Is%20Valid
      _)
    (:Is%20Not%20Valid
      (bind _returnvalue (UserInterface|CreateWidget "/Game/Widget/WB_Beccati.WB_Beccati_C" self))
      (Variables|Default|SetWB_UI_Death_All _returnvalue)))
  (UserInterface|Viewport|AddtoViewport (Variables|Default|GetWB_UI_Death_All) 0)
  (Utilities|FlowControl|Delay 3.0)
  (Widget|RemovefromParent (Variables|Default|GetWB_UI_Death_All)))

(event EventBeginPlay
  (if (Pawn|IsLocalPlayerController)
    ;[1 1 1] Attivazione del sistema avanzato di gestione dell'input
    (Input|AddMappingContext (PlayerController|LocalPlayerSubsystems|GetEnhancedInputLocalPlayerSubsystem) "/Game/Input/IMC_Input.IMC_Input" 0 "(bIgnoreAllPressedKeysUntilRelease=True,bForceImmediately=False,bNotifyUserSettings=False)")
    (Viewport|RemoveAllWidgets)
    (CallFunction|UIShowinGameHUD)
    (Input|SetInputModeGameOnly self false)
    (Variables|Default|SetbShowMouseCursor false)))

(fn ConstructionScript)

(fn UIShowinGameHUD
  (Utilities|IsValid (Variables|Default|GetWB_IngameHUD)
    (:Is%20Valid
      _)
    (:Is%20Not%20Valid
      (bind _returnvalue (UserInterface|CreateWidget "/Game/Widget/WB_InagameHUD.WB_InagameHUD_C" self))
      (Variables|Default|SetWB_IngameHUD _returnvalue)))
  (UserInterface|Viewport|AddtoViewport (Variables|Default|GetWB_IngameHUD) 0)
  (return))