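; Menu game mode that tracks connected players in the lobby and shares their profiles.
; New players on the lobby map are added to a menu controller list, then after a short delay get their lobby menu and initial setup.
; UpdateLobby copies each controller's profile to its PlayerState and sends the full profile list to every controller.
; Logout removes the controller and triggers the same refresh.
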(event Custom|UpdateLobby
  (params (PlayerNames :type Boolean))
  ;[1 1 1] UpdateLobby. Add all players names to the lobby
  (if PlayerNames
    (Utilities|Array|Clear (Variables|Default|GetAll_PlayerProfiles))
    (for _array_element (Variables|Default|GetAll_ConnectedPlayer)
      (Utilities|Array|Add (Variables|Default|GetAll_PlayerProfiles) (Variables|/Game/Blueprints/FrameWork/Menu/BP_MenuController.BP_MenuController_C|GetPlayerProfileInfo _array_element))
      (bind _asbp_player_state (Utilities|Casting|CastToBP_PlayerState (Variables|/Script/Engine.Controller|GetPlayerState _array_element)))
      (Variables|/Game/Blueprints/FrameWork/BP_PlayerState.BP_PlayerState_C|SetS_PlayerProfile _asbp_player_state (Variables|/Game/Blueprints/FrameWork/Menu/BP_MenuController.BP_MenuController_C|GetPlayerProfileInfo _array_element)))
    (for _array_element_2 (Variables|Default|GetAll_ConnectedPlayer)
      (if PlayerNames
        (Default|UpdatePlayerNames _array_element_2 (Variables|Default|GetAll_PlayerProfiles))))))

(event EventHandleStartingNewPlayer
  (params (NewPlayer :type Player%20Controller%20Object%20Reference))
  ;[1 1 1] When a new player is connecting
  (bind _returnvalue (Game|GetCurrentLevelName true))
  (switch string _returnvalue
    (:LobbyMenuMap
      (bind _asbp_menu_controller (Utilities|Casting|CastToBP_MenuController NewPlayer))
      (Utilities|Array|Add (Variables|Default|GetAll_ConnectedPlayer) _asbp_menu_controller)
      (Utilities|FlowControl|Delay 0.1)
      (Default|CreateLobbyMenu _asbp_menu_controller)
      (Default|InitialSetup _asbp_menu_controller))))

(event EventOnLogout
  (params (ExitingController :type Controller%20Object%20Reference))
  ;[1 1 1] Event OnLogout
  (bind _asbp_menu_controller (Utilities|Casting|CastToBP_MenuController ExitingController))
  (Utilities|Array|RemoveItem (Variables|Default|GetAll_ConnectedPlayer) _asbp_menu_controller)
  (CallFunction|UpdateLobby true))

(fn ConstructionScript)