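; Player controller for the menu and lobby that sets UI-only input with a visible cursor and manages the lobby and loading screen widgets.
; Initial setup loads or creates the saved player profile, then sends it through a server update event so BP_MenuGameMode refreshes the lobby.
; Other events push player names into the lobby widget, show the load screen, or destroy the session and return to the main menu map.
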(event Custom|EndClientSession
  ;[1 1 1] End Client Session
  (|DestroySession self
    (:then
      (Game|OpenLevel(byName) "MainMenuMap"))))

(event Custom|CreateLobbyMenu
  ;[1 1 1] CreateLobbymenuEvent. Show Lobby Menu
  (CallFunction|UIShowLobbyMenu))

(event Custom|CreateLoadScreen
  ;[1 1 1] Create Load Screen
  (CallFunction|UIShowLoadScreen))

(event Custom|Initial_Setup
  ;[1 1 1] Initial_Setup.  Update Lobby
  (CallFunction|LoadSavedProfile)
  (CallFunction|ServerUpdateLobby (Variables|Default|GetPlayerProfileInfo)))

(event Custom|UpdatePlayerNames
  (params (PlayerProfiles :type Array%20of%20S%20Player%20Profile%20Structures))
  (bind _wb_lobbymenu (Variables|Default|GetWB_LobbyMenu))
  ;[1 1 1] Update PLayer Names in Lobby menu
  (Utilities|IsValid _wb_lobbymenu
    (:Is%20Valid
      (Default|ClearPlayerNames _wb_lobbymenu)
      (Default|UpdatePlayerNames _wb_lobbymenu PlayerProfiles))))

(event Custom|Server_UpdateLobby
  (params (PlayerProfile :type S%20Player%20Profile%20Structure))
  ;[1 1 1] Initial_Setup.  Update Lobby
  (Variables|Default|SetPlayerProfileInfo PlayerProfile)
  (bind _asbp_menu_game_mode (Utilities|Casting|CastToBP_MenuGameMode (Game|GetGameMode)))
  (Default|UpdateLobby _asbp_menu_game_mode true))

(event EventBeginPlay
  ;[1 1 1] Event BeginPlay. Set input on UI only
  (if (Pawn|IsLocalController)
    (Variables|Default|SetbShowMouseCursor true)
    (Input|SetInputModeUIOnly self 0 "DoNotLock" false)))

(fn ConstructionScript)

(fn UIShowLobbyMenu
  (Utilities|IsValid (Variables|Default|GetWB_LobbyMenu)
    (:Is%20Valid
      _)
    (:Is%20Not%20Valid
      (bind _returnvalue (UserInterface|CreateWidget "/Game/Widget/WB_LobbyMenu.WB_LobbyMenu_C" self))
      (Variables|Default|SetWB_LobbyMenu _returnvalue)))
  (UserInterface|Viewport|AddtoViewport (Variables|Default|GetWB_LobbyMenu) 0)
  (return))

(fn LoadSavedProfile
  (bind _returnvalue (SaveGame|DoesSaveGameExist (LocalVariables|GetLcl_Slot%20Name)))
  (if _returnvalue
    _
    (else
      (bind _returnvalue_2 (SaveGame|CreateSaveGameObject "/Game/SavedData/SG_PlayerProfile.SG_PlayerProfile_C"))
      (SaveGame|SaveGametoSlot _returnvalue_2 (LocalVariables|GetLcl_Slot%20Name))))
  (bind _returnvalue_3 (SaveGame|LoadGamefromSlot (LocalVariables|GetLcl_Slot%20Name)))
  (bind _assg_player_profile (Utilities|Casting|CastToSG_PlayerProfile _returnvalue_3))
  (Variables|Default|SetPlayerProfileInfo (Variables|/Game/SavedData/SG_PlayerProfile.SG_PlayerProfile_C|GetPlayerProfile _assg_player_profile))
  (return))

(fn UIShowLoadScreen
  (Viewport|RemoveAllWidgets)
  (Utilities|IsValid (Variables|Default|GetWB_LoadScreen)
    (:Is%20Valid
      _)
    (:Is%20Not%20Valid
      (bind _returnvalue (UserInterface|CreateWidget "/Game/Widget/WB_LoadScreen.WB_LoadScreen_C" self))
      (Variables|Default|SetWB_LoadScreen _returnvalue)))
  (UserInterface|Viewport|AddtoViewport (Variables|Default|GetWB_LoadScreen) 0)
  (return))