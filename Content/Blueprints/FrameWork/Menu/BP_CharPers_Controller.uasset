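; Player controller for the character personalization menu, which previews the player's chosen model on the level's BP_Character under UI-only input.
; BeginPlay applies the current profile's mesh via a CharModelInfo_Table lookup, while separate events create the widget and load or create the profile save.
; SaveSelectedCharacter updates the profile, delegates saving to BP_GameInstance and refreshes the mesh.
; An in-controller save path is left disconnected, noted as not working.
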(event Custom|UpdateSelectedChar
  (params (PlayerProfile :type S%20Player%20Profile%20Structure))
  (bind _returnvalue (Utilities|GetDataTableRow "/Game/Characters/Character/CharModelInfo_Table.CharModelInfo_Table" (.skeletalmesh PlayerProfile))
    (:then
      (Default|SetCharMesh (Variables|Default|GetBP_CharSelection) (Utilities|Struct|BreakS_CharModelInfo _returnvalue)))))

(event Custom|Initial_Setup
  (CallFunction|LoadSavedProfile))

(event Custom|setSavedModel
  (CallFunction|UpdateSelectedChar (Variables|Default|GetPlayerProfileInfo)))

(event Custom|CreatePersonalizationMenu
  (CallFunction|UICharPersMenu))

(event EventBeginPlay
  ;[1 1 1] Event BeginPlay. Set input on UI only
  (bind _asbp_game_instance (Utilities|Casting|CastToBP_GameInstance (Game|GetGameInstance)))
  (Variables|Default|SetAs%20BP%20Game%20Instance _asbp_game_instance)
  (bind _returnvalue (Actor|GetActorOfClass "/Game/Blueprints/CharPersonalization/BP_Character.BP_Character_C"))
  (Variables|Default|SetBP_CharSelection _returnvalue)
  (CallFunction|SetSavedModel)
  (Variables|Default|SetbShowMouseCursor true)
  (Input|SetInputModeUIOnly self 0 "DoNotLock" false))

(fn ConstructionScript)

(fn UICharPersMenu
  (Utilities|IsValid (Variables|Default|GetWB_CharPersonlazation)
    (:Is%20Valid
      _)
    (:Is%20Not%20Valid
      (bind _returnvalue (UserInterface|CreateWidget "/Game/Widget/WB_CharPersonalization.WB_CharPersonalization_C" self))
      (Variables|Default|SetWB_CharPersonlazation _returnvalue)))
  (UserInterface|Viewport|AddtoViewport (Variables|Default|GetWB_CharPersonlazation) 0)
  (return))

(fn LoadSavedProfile
  (bind _returnvalue (SaveGame|DoesSaveGameExist (LocalVariables|GetLcl_Slot%20Name)))
  (if _returnvalue
    _
    (else
      (bind _returnvalue_2 (SaveGame|CreateSaveGameObject "/Game/SavedData/SG_PlayerProfile.SG_PlayerProfile_C"))
      (SaveGame|SaveGametoSlot _returnvalue_2 (LocalVariables|GetLcl_Slot%20Name))))
  (bind _returnvalue_3 (SaveGame|LoadGamefromSlot (LocalVariables|GetLcl_Slot%20Name)))
  (bind _assg_player_profile (Utilities|Casting|CastToSG_PlayerProfile _returnvalue_3))
  (Variables|Default|SetPlayerProfileInfo (Variables|/Game/SavedData/SG_PlayerProfile.SG_PlayerProfile_C|GetPlayerProfile _assg_player_profile))
  (return))

(fn SaveSelectedCharacter
  (params (RawName :type Name))
  (Variables|Default|SetPlayerProfileInfo (Utilities|Struct|MakeS_PlayerProfile (.playername (Variables|Default|GetPlayerProfileInfo)) RawName))
  (Default|SaveCharModel (Variables|Default|GetAs%20BP%20Game%20Instance) (Variables|Default|GetPlayerProfileInfo))
  (CallFunction|UpdateSelectedChar (Variables|Default|GetPlayerProfileInfo))
  (return))