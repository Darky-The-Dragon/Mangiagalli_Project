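; BP_Inn is the inn location on the game map, which lets the local player know they can go back into the inn.
; A box trigger reacts only to a locally controlled BP_Player_GameMap, sending it a near-level message with "Inn_Level" on entry and clearing it on exit.
; It also shows a tap-E prompt widget, created once and reused, and removes it when the player leaves.
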(event OnComponentBeginOverlap(Box)
  (params (OverlappedComponent :type Primitive%20Component%20Object%20Reference) (OtherActor :type Actor%20Object%20Reference) (OtherComp :type Primitive%20Component%20Object%20Reference) (OtherBodyIndex :type Integer) (bFromSweep :type Boolean) (SweepResult :type Hit%20Result%20Structure%20%28by%20ref%29))
  (bind _asbp_player_game_map (Utilities|Casting|CastToBP_Player_GameMap OtherActor))
  (if (Pawn|IsLocallyControlled _asbp_player_game_map)
    (Class|BPIIconLevel|IsNearLevel(Message) OtherActor true "Inn_Level")
    (Utilities|IsValid (Variables|Default|GetWB_GoBackInn)
      (:Is%20Valid
        _)
      (:Is%20Not%20Valid
        (bind _returnvalue (UserInterface|CreateWidget "/Game/Widget/WB_TapEToGoBackInn.WB_TapEToGoBackInn_C" (Pawn|GetLocalViewingPlayerController _asbp_player_game_map)))
        (Variables|Default|SetWB_GoBackInn _returnvalue)))
    (UserInterface|Viewport|AddtoViewport (Variables|Default|GetWB_GoBackInn) 0)
    (Development|PrintString "NearInn")))

(event OnComponentEndOverlap(Box)
  (params (OverlappedComponent :type Primitive%20Component%20Object%20Reference) (OtherActor :type Actor%20Object%20Reference) (OtherComp :type Primitive%20Component%20Object%20Reference) (OtherBodyIndex :type Integer))
  (bind _asbp_player_game_map (Utilities|Casting|CastToBP_Player_GameMap OtherActor))
  (if (Pawn|IsLocallyControlled _asbp_player_game_map)
    (Class|BPIIconLevel|IsNearLevel(Message) OtherActor false)
    (Utilities|IsValid (Variables|Default|GetWB_GoBackInn)
      (:Is%20Valid
        (Widget|RemovefromParent (Variables|Default|GetWB_GoBackInn))
        (Development|PrintString "Not near Inn")))))

(event EventBeginPlay)

(event Collision|EventActorBeginOverlap
  (params (OtherActor :type Actor%20Object%20Reference)))

(event EventTick
  (params (DeltaSeconds :type Float%20%28single-precision%29)))

(fn ConstructionScript)