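; Golgi dartboard target that scores hits on its cylinder by how close they land to the actor's center.
; A chain of float comparisons on impact distance sorts each hit into concentric bands, adding more points nearer the center.
; The last comparison tests a constant zero instead of distance, so any hit beyond the outer threshold still scores the minimum.
; The running total resets at BeginPlay and prints after scoring.
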(event OnComponentHit(Bersaglio_Golgi_Cilindro)
  (params (HitComponent :type Primitive%20Component%20Object%20Reference) (OtherActor :type Actor%20Object%20Reference) (OtherComp :type Primitive%20Component%20Object%20Reference) (NormalImpulse :type Vector :default "0, 0, 0") (Hit :type Hit%20Result%20Structure%20%28by%20ref%29))
  (bind _returnvalue (Transformation|GetActorLocation))
  (bind _returnvalue_2 (Math|Vector|Distance(Vector) _returnvalue (.impactpoint Hit)))
  (Math|Float|CompareFloat _returnvalue_2 8e+01
    (:>
      (Math|Float|CompareFloat _returnvalue_2 1.6e+02
        (:>
          (Math|Float|CompareFloat _returnvalue_2 2.4e+02
            (:>
              (Math|Float|CompareFloat _returnvalue_2 3.2e+02
                (:>
                  (Math|Float|CompareFloat 0.0 4e+02
                    (:>
                      _)
                    (:<
                      (Variables|Default|Setpoints (+ (Variables|Default|Getpoints) 2.0)))))
                (:<
                  (Variables|Default|Setpoints (+ (Variables|Default|Getpoints) 4.0)))))
            (:<
              (Variables|Default|Setpoints (+ (Variables|Default|Getpoints) 6.0)))))
        (:<
          (Variables|Default|Setpoints (+ (Variables|Default|Getpoints) 8.0)))))
    (:<
      (bind _output_get (Variables|Default|Setpoints (+ (Variables|Default|Getpoints) 1e+01)))))
  (Development|PrintString (Utilities|String|ToString(Float) _output_get)))

(event EventBeginPlay
  (Variables|Default|Setpoints 0.0))

(fn ConstructionScript)