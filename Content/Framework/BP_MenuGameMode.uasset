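; BP_MenuGameMode is the menu game mode that manages players joining the lobby and their shared profile list.
; On the Lobby Menu Map, HandleStartingNewPlayer registers each BP_MenuController, has it create the lobby menu and runs its initial setup.
; UpdateLobby, when its PlayerNames flag is set, rebuilds the profile list from all connected controllers and passes it back to each to update player names.
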(event Custom|UpdateLobby
  (params (PlayerNames :type Boolean))
  (if PlayerNames
    (Utilities|Array|Clear (Variables|Default|GetAll_PlayerProfiles))
    (for _array_element (Variables|Default|GetAll_ConnectedPlayer)
      (Utilities|Array|Add (Variables|Default|GetAll_PlayerProfiles) (Variables|/Game/Framework/BP_MenuController.BP_MenuController_C|GetPlayerProfileInfo _array_element)))
    (for _array_element_2 (Variables|Default|GetAll_ConnectedPlayer)
      (if PlayerNames
        (Default|UpdatePlayerNames _array_element_2 (Variables|Default|GetAll_PlayerProfiles))))))

(event EventBeginPlay)

(event EventTick
  (params (DeltaSeconds :type Float%20%28single-precision%29)))

(event EventHandleStartingNewPlayer
  (params (NewPlayer :type Player%20Controller%20Object%20Reference))
  (bind _returnvalue (Game|GetCurrentLevelName true))
  (switch string _returnvalue
    (:LobbyMenuMap
      (bind _asbp_menu_controller (Utilities|Casting|CastToBP_MenuController NewPlayer))
      (Utilities|Array|Add (Variables|Default|GetAll_ConnectedPlayer) _asbp_menu_controller)
      (Default|CreateLobbyMenuEvent _asbp_menu_controller)
      (Default|InitialSetup _asbp_menu_controller))))

(fn ConstructionScript)