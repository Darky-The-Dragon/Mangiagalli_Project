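; BP_MenuController is a player controller for menus that sets up UI input and shows the lobby menu.
; On BeginPlay, the local controller shows the mouse cursor and switches to UI-only input.
; CreateLobbyMenuEvent calls a function that creates WB_LobbyMenu behind a validity check, stores it and adds it to the viewport.
; EndClientSession destroys the online session, then opens MainMenuMap.
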(event Custom|EndClientSession
  (|DestroySession self
    (:then
      (Game|OpenLevel(byName) "MainMenuMap"))))

(event Custom|CreateLobbyMenuEvent
  (CallFunction|UIShowLobbyMenu))

(event EventTick
  (params (DeltaSeconds :type Float%20%28single-precision%29)))

(event EventBeginPlay
  (if (Pawn|IsLocalController)
    (Variables|Default|SetbShowMouseCursor true)
    (Input|SetInputModeUIOnly self 0 "DoNotLock" false)))

(fn ConstructionScript)

(fn UIShowLobbyMenu
  (Utilities|IsValid 0
    (:Is%20Valid
      _)
    (:Is%20Not%20Valid
      (bind _returnvalue (UserInterface|CreateWidget "/Game/Widget/WB_LobbyMenu.WB_LobbyMenu_C" self))
      (Variables|Default|SetWB_LobbyMenu _returnvalue)))
  (UserInterface|Viewport|AddtoViewport (Variables|Default|GetWB_LobbyMenu) 0)
  (return))