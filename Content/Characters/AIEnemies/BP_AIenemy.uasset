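; Mafia enemy AI that uses PawnSensing to catch players, as either a chaser or a stationary spotter, chosen by the Search flag.
; Chasers run after seen players, sprinting when far and slowing within range, where reaching one triggers a catch.
; Spotters catch on sight, briefly disabling sight afterwards.
; Catches respawn all players through BP_GameMode and reset companion positions; roam and fixed-move events go uncalled here.
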(event OnSeePawn(PawnSensing)
  (params (Pawn :type Pawn%20Object%20Reference))
  (if (Variables|Default|GetSearch)
    (Utilities|FlowControl|Sequence
      (:then_0
        (bind _asbp_player (Utilities|Casting|CastToBP_Player Pawn))
        (CallFunction|CalculateDistancefromPlayer _asbp_player)
        (if (> (Variables|Default|GetDistanceFromPlayer) 1e+03)
          (bind _output_get (Variables|/Script/Engine.CharacterMovementComponent|SetMaxWalkSpeed (Variables|Character|GetCharacterMovement) 1.2e+03))
          (Development|PrintString (Utilities|String|ToString(Float) _output_get))
          (AI|AIMoveTo self "0, 0, 0" Pawn 0.0 true)
          (else
            (bind _output_get_2 (Variables|/Script/Engine.CharacterMovementComponent|SetMaxWalkSpeed (Variables|Character|GetCharacterMovement) 6.5e+02))
            (Development|PrintString (Utilities|String|ToString(Float) _output_get_2))
            (AI|AIMoveTo self "0, 0, 0" Pawn 0.0 true
              (:OnSuccess
                ;[1 1 1] When Mafia inseguitrice recheas us
                (bind _asbp_game_mode (Utilities|Casting|CastToBP_GameMode (Game|GetGameMode)))
                (Default|RespawnAllPlayers _asbp_game_mode (Transformation|GetActorTransform (Variables|Default|GetRespawnLocationForPlayers)))
                (Utilities|FlowControl|Delay 3.0)
                (CallFunction|ResetPosition)
                (for _array_element (Variables|Default|GetAI_Mafia_Companion)
                  (CallFunction|ResetPosition _array_element)
                  (Default|ResetRespawn _asbp_game_mode))))))))
    (else
      ;[1 1 1] PawnFermo che sgama il giocatore
      (Variables|/Script/AIModule.PawnSensingComponent|SetbSeePawns (Variables|Default|GetPawnSensing) false)
      (CallFunction|Sgamato)
      (Utilities|FlowControl|Delay 3.0)
      (Variables|/Script/AIModule.PawnSensingComponent|SetbSeePawns (Variables|Default|GetPawnSensing) true))))

(event Custom|Random%20Roam
  (AI|AIMoveTo self (.RandomLocation (AI|Navigation|GetRandomReachablePointinRadius (Transformation|GetActorLocation) 2e+02 0 0)) 0 5.0 false
    (:OnSuccess
      (CallFunction|RandomRoam))))

(event Custom|CalculateDistanceFromPlayer
  (params (Pawn :type Pawn%20Object%20Reference))
  (Variables|Default|SetDistanceFromPlayer (Math|Float|Absolute(Float) (Math|Vector|Distance(Vector) (Transformation|GetActorLocation) (Transformation|GetActorLocation Pawn)))))

(event Custom|MoveToPos
  (AI|AIMoveTo self "1778.000000,-6688.000000,0.000000" 0 0.0 true
    (:OnSuccess
      (Development|PrintString "Posizione raggiunta"))))

(event Custom|ResetPosition
  ;[1 1 1] Reset Position
  (Transformation|SetActorTransform (Transformation|GetActorTransform (Variables|Default|GetInitialPosition)) false true))

(event Custom|Sgamato
  ;[1 1 1] Sgamato. Respawn all players e MafiaInseguitrice, e resetta la morte
  (Development|PrintString "Sgamato")
  (bind _asbp_game_mode (Utilities|Casting|CastToBP_GameMode (Game|GetGameMode)))
  (Default|RespawnAllPlayers _asbp_game_mode (Transformation|GetActorTransform (Variables|Default|GetRespawnLocationForPlayers)))
  (for _array_element (Variables|Default|GetAI_Mafia_Companion)
    (CallFunction|ResetPosition _array_element))
  (Default|ResetRespawn _asbp_game_mode))

(fn ConstructionScript)