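; BP_PlaceHolderLobby is a character Blueprint holding helper logic for ledge detection and hanging.
; SetLedgeTraceResult validates the hit actor, checks its "Hangable" tag, and builds a target transform from the impact point, offset by height and forward vector, keeping the actor's rotation.
; A Movement Mode macro sets movement, collision on the mesh, Remy and capsule, and the hanging flag.
; PrintDebug prints joined strings; no event graph appears here.
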(fn ConstructionScript)

(fn SetLedgeTraceResult
  (params (DidHitLedge? :type Boolean) (ImpactPointIn :type Vector) (ImpactPointNormalIn :type Vector) (HitActorIn :type Actor%20Object%20Reference) (AdjustCharacterHeight :type Float%20%28double-precision%29) (AdjustCharacterForward :type Float%20%28double-precision%29))
  (bind _returnvalue (Transformation|GetActorRotation))
  (bind _returnvalue_2 (Transformation|GetActorForwardVector))
  (bind _returnvalue_3 (* _returnvalue_2 AdjustCharacterForward))
  (Utilities|IsValid HitActorIn
    (:Is%20Valid
      ;[1 1 1] Set
      (Variables|Default|SetDid%20Hit%20Ledge? DidHitLedge?)
      (Variables|Default|SetisHangable? (Actor|ActorHasTag HitActorIn "Hangable"))
      (Variables|Default|SetHit%20Actor HitActorIn)
      (Variables|Default|SetImpact%20Point ImpactPointIn)
      (Variables|Default|SetActor%20Transform (Transformation|GetActorTransform))
      (Variables|Default|SetTarget%20Transform (Math|Transform|MakeTransform (+ (Math|Vector|MakeVector (.x _returnvalue_3) (.y _returnvalue_3) 0.0) (Math|Vector|MakeVector (.X (Math|Vector|BreakVector (Variables|Default|GetImpact%20Point))) (.Y (Math|Vector|BreakVector (Variables|Default|GetImpact%20Point))) (- (.Z (Math|Vector|BreakVector (Variables|Default|GetImpact%20Point))) AdjustCharacterHeight))) (Math|Rotator|MakeRotator (.roll _returnvalue) (.pitch _returnvalue) (.Yaw (Math|Rotator|BreakRotator (Transformation|GetActorRotation))))))
      (return (Variables|Default|GetTarget%20Transform) (Variables|Default|GetActor%20Transform)))
    (:Is%20Not%20Valid
      (Variables|Default|SetDid%20Hit%20Ledge? false)
      (Variables|Default|SetisHangable? false))))